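; Mole actor (Topo) that repeatedly rises and hides, apparently for a whack-a-mole style game.
; The ArribaAbajo timeline moves the mesh on Z after a random delay, then reverses after a shorter random wait.
; The Escondido flag alternates the timeline's Finished branch between lowering and restarting the cycle.
; At BeginPlay and after each descent, a coin flip picks sheep or cow fur and sets IsEnemy accordingly.
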(event Custom|EventoAbajo
  (Utilities|FlowControl|Delay (Math|Random|RandomFloatinRange 0.0 1.0))
  (bind _z_topo (Timeline|ArribaAbajo ReverseFromEnd)
    (:Update
      (Transformation|SetRelativeLocation (Variables|Default|GetTopo) (Math|Vector|MakeVector 0.0 0.0 _z_topo) false false))
    (:Finished
      (if (Variables|Default|GetEscondido?)
        (Variables|Default|SetEscondido? false)
        (CallFunction|EventoAbajo)
        (else
          (Variables|Default|SetEscondido? true)
          (if (Math|Random|RandomBool)
            (Rendering|Material|SetMaterial (Variables|Default|GetTopo) 0 "/Game/Materiales/Tileable_Sheep_Fur_skmaxwl/Tileable_Sheep_Fur_skmaxwl_inst.Tileable_Sheep_Fur_skmaxwl_inst")
            (Variables|Default|SetisEnemy true)
            (else
              (Rendering|Material|SetMaterial (Variables|Default|GetTopo) 0 "/Game/Materiales/Cow_Fur_rlpuprp0/Cow_Fur_rlpuprp0_inst.Cow_Fur_rlpuprp0_inst")
              (Variables|Default|SetisEnemy false)))
          (CallFunction|EventoArriba))))))

(event Custom|EventoArriba
  (Utilities|FlowControl|Delay (Math|Random|RandomFloatinRange 4.0 6.0))
  (bind _z_topo (Timeline|ArribaAbajo Play)
    (:Update
      (Transformation|SetRelativeLocation (Variables|Default|GetTopo) (Math|Vector|MakeVector 0.0 0.0 _z_topo) false false))
    (:Finished
      (if (Variables|Default|GetEscondido?)
        (Variables|Default|SetEscondido? false)
        (CallFunction|EventoAbajo)
        (else
          (Variables|Default|SetEscondido? true)
          (if (Math|Random|RandomBool)
            (Rendering|Material|SetMaterial (Variables|Default|GetTopo) 0 "/Game/Materiales/Tileable_Sheep_Fur_skmaxwl/Tileable_Sheep_Fur_skmaxwl_inst.Tileable_Sheep_Fur_skmaxwl_inst")
            (Variables|Default|SetisEnemy true)
            (else
              (Rendering|Material|SetMaterial (Variables|Default|GetTopo) 0 "/Game/Materiales/Cow_Fur_rlpuprp0/Cow_Fur_rlpuprp0_inst.Cow_Fur_rlpuprp0_inst")
              (Variables|Default|SetisEnemy false)))
          (CallFunction|EventoArriba))))))

(event Custom|TipoTopo
  (if (Math|Random|RandomBool)
    (Rendering|Material|SetMaterial (Variables|Default|GetTopo) 0 "/Game/Materiales/Tileable_Sheep_Fur_skmaxwl/Tileable_Sheep_Fur_skmaxwl_inst.Tileable_Sheep_Fur_skmaxwl_inst")
    (Variables|Default|SetisEnemy true)
    (else
      (Rendering|Material|SetMaterial (Variables|Default|GetTopo) 0 "/Game/Materiales/Cow_Fur_rlpuprp0/Cow_Fur_rlpuprp0_inst.Cow_Fur_rlpuprp0_inst")
      (Variables|Default|SetisEnemy false)))
  (CallFunction|EventoArriba))

(event EventBeginPlay
  (CallFunction|EventoArriba)
  (CallFunction|TipoTopo))

(fn ConstructionScript)